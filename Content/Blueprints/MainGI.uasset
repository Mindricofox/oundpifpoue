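; MainGI, apparently the Game Instance, handles multiplayer session hosting and joining along with the menus for both.
; ShowSearch and HostGameMenu lazily create, cache and show the SearchGames and HostGame widgets.
; Launch stores the server name, creates a session as LAN or online based on the Steam flag, then opens the game level as a listen server.
; Join joins a given search result, and both session calls print on failure.
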(event `Join`
  (params (Session :type "BlueprintSessionResult Structure"))
  (`JoinSessionCallbackProxy.JoinSession` (`GameplayStatics.GetPlayerController` 0) Session
    (:`OnFailure`
      (`KismetSystemLibrary.PrintString` "FAILED"))))

(event `ShowSearch`
  (`/Engine/EditorBlueprintResources/StandardMacros.IsValid` (`self.Search`)
    (:`Is Valid`
      _)
    (:`Is Not Valid`
      (bind _returnvalue (`|CreateWidget` "/Game/UI/SearchGames.SearchGames_C" (`GameplayStatics.GetPlayerController` 0)))
      (bind _output_get (set `self.Search` _returnvalue))))
  (`UserWidget.AddToViewport` _output_get 0))

(event `HostGameMenu`
  (`/Engine/EditorBlueprintResources/StandardMacros.IsValid` (`self.Host`)
    (:`Is Valid`
      _)
    (:`Is Not Valid`
      (bind _returnvalue (`|CreateWidget` "/Game/UI/HostGame.HostGame_C" (`GameplayStatics.GetPlayerController` 0)))
      (bind _output_get (set `self.Host` _returnvalue))))
  (`UserWidget.AddToViewport` _output_get 0))

(event `Launch`
  (params (`Steam?` :type Boolean) (ServerName :type Text))
  (set `self.Name` ServerName)
  (`CreateSessionCallbackProxy.CreateSession` (`GameplayStatics.GetPlayerController` 0) 8 (not `Steam?`)
    (:`OnSuccess`
      (`GameplayStatics.OpenLevel` "BestWorlInTheWorld" true "listen"))
    (:`OnFailure`
      (`KismetSystemLibrary.PrintString` "FAILED"))))